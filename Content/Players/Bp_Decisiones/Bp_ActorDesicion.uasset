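; Decision trigger actor that opens a three-option dialogue widget when the player enters its Box.
; On overlap it fills BpWidgetDesicion with dialogue and option text, shows the cursor, switches to UI-only input and disables the player character's input.
; The widget's exit dispatcher is bound to DecisiontEvent, which re-broadcasts through the actor's own DecisionDispatcher.
; End overlap hides the TextRender; the timed TakeDamage event is an empty stub.
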(event `DecisiontEvent`
  (`self.DecisionDispatcher`))

(event `self.Box.OnComponentBeginOverlap`
  (params (OverlappedComponent :type "PrimitiveComponent Object Reference") (OtherActor :type "Actor Object Reference") (OtherComp :type "PrimitiveComponent Object Reference") (OtherBodyIndex :type Integer) (bFromSweep :type Boolean) (SweepResult :type "HitResult Structure (by ref)"))
  (bind _returnvalue (`GameplayStatics.GetPlayerController` 0))
  (bind _dialogue_widget (`self.Dialogue Widget`))
  (if (`self.ActorHasTag` OtherActor "Player")
    (`KismetSystemLibrary.K2_SetTimerDelegate` (delegate `TakeDamage`) 1.0)
    (cast `/Game/Players/Bp/PlayerBp` OtherActor)
    (`self.EnableInput` (`GameplayStatics.GetPlayerController` 0))
    (bind _returnvalue_2 (`|CreateWidget` "/Game/Widgest/BpWidgetDesicion.BpWidgetDesicion_C"))
    (bind _output_get (set `self.Dialogue Widget` _returnvalue_2))
    (`TextBlock.SetText` (`/Game/Widgest/BpWidgetDesicion.textDialogue` (`self.Dialogue Widget`)) (`|GetArrayItem` (`self.Dialogue Text`) (`self.index`)))
    (`TextBlock.SetText` (`/Game/Widgest/BpWidgetDesicion.TextOption1` _dialogue_widget) (`self.TextOption`))
    (`TextBlock.SetText` (`/Game/Widgest/BpWidgetDesicion.TextOption2` _dialogue_widget) (`self.TextOption2`))
    (`TextBlock.SetText` (`/Game/Widgest/BpWidgetDesicion.TextOption3` _dialogue_widget) (`self.TextOption3`))
    (`UserWidget.AddToViewport` _output_get 0)
    (add `/Game/Widgest/BpWidgetDesicion.ExitDispatcher` _returnvalue_2 (delegate `DecisiontEvent`))
    (set `PlayerController.bShowMouseCursor` true _returnvalue)
    (`WidgetBlueprintLibrary.SetInputMode_UIOnlyEx` _returnvalue _returnvalue_2)
    (bind _asplayer_bp (cast `/Game/Players/Bp/PlayerBp` (`GameplayStatics.GetPlayerCharacter` 0)))
    (`self.DisableInput` _asplayer_bp _returnvalue)))

(event `TakeDamage`)

(event `self.Box.OnComponentEndOverlap`
  (params (OverlappedComponent :type "PrimitiveComponent Object Reference") (OtherActor :type "Actor Object Reference") (OtherComp :type "PrimitiveComponent Object Reference") (OtherBodyIndex :type Integer))
  (cast `/Game/Players/Bp/PlayerBp` OtherActor)
  (`self.EnableInput` (`GameplayStatics.GetPlayerController` 0))
  (`SceneComponent.SetHiddenInGame` (`self.TextRender`) true false)
  (`/Engine/EditorBlueprintResources/StandardMacros.IsValid` null))

(fn `UserConstructionScript`)