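; Player Blueprint that handles top-down-style movement and interaction with nearby actors.
; BeginPlay adds the Enhanced Input mapping context and creates the main UI widget.
; Move input drives world-axis movement and stores the direction.
; One interaction input takes a bp_actor1's Recoleccion result from the collision box and shows it as widget dialogue; another sends a dialogue message to the first overlapping Dialog_Interface actor.
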(event `self.ReceiveBeginPlay`
  ; Configurar Teclas
  (`|ExecutionSequence`
    (:`then_0`
      (bind _asplayer_controller (cast `PlayerController` (`self.GetController`)))
      (`EnhancedInputSubsystemInterface.AddMappingContext` (pcsubsystem `EnhancedInputLocalPlayerSubsystem` _asplayer_controller) "/Game/Players/Bp/PlayerMapping.PlayerMapping" 0 (struct)))
    (:`then_1`
      (bind _returnvalue (`|CreateWidget` "/Game/Widgest/BPWidgetMain.BPWidgetMain_C"))
      (`UserWidget.AddToViewport` _returnvalue 0)
      (set `self.mainWidget` _returnvalue))))

(event `EnhancedInput|/Game/Players/Bp/LP_interaccion`
  (params (ActionValue :type Boolean) (ElapsedSeconds :type "Float (double-precision)") (TriggeredSeconds :type "Float (double-precision)") (InputAction :type "InputAction Object Reference" :default "/Game/Players/Bp/LP_interaccion.LP_interaccion"))
  (:`Triggered`
    (for _array_element (`PrimitiveComponent.GetOverlappingActors` (`self.BoxCollision`) null)
      (bind _asbp_actor_1 (cast `/Game/Players/Bp/Bp_interface/bp_actor1` _array_element))
      (bind _mensaje (`/Game/Players/Bp/Bp_interface/bp_actor1.Recoleccion` _asbp_actor_1))
      (`/Game/Widgest/BPWidgetMain.MostrarDialogo` (`self.mainWidget`) _mensaje)
      (break))))

(event `EnhancedInput|/Game/Players/Bp/PlayerMove`
  (params (ActionValue :type "Vector2D Structure") (ElapsedSeconds :type "Float (double-precision)") (TriggeredSeconds :type "Float (double-precision)") (InputAction :type "InputAction Object Reference" :default "/Game/Players/Bp/PlayerMove.PlayerMove"))
  ; ControlarMovimientoJugador
  (:`Triggered`
    (`self.AddMovementInput` (1.0 0.0 0.0) ActionValue_X)
    (`self.AddMovementInput` (0.0 -1.0 0.0) ActionValue_Y)
    (set `self.Direccion` (`KismetMathLibrary.MakeVector2D` ActionValue_X ActionValue_Y))))

(event `InputAction|Interacte`
  (params (Key :type "Key Structure"))
  (:`Pressed`
    (for _array_element (`self.GetOverlappingActors` null)
      (if (`KismetSystemLibrary.DoesImplementInterface` _array_element "/Game/Players/Bp/Bp_interface/Dialog_Interface.Dialog_Interface_C")
        (message `/Game/Players/Bp/Bp_interface/Dialog_Interface.EventDialog` _array_element)
        (break)))))

(fn `UserConstructionScript`)