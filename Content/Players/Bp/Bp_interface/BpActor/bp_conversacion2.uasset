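; Dialogue trigger actor that steps the player through an array of text lines using an interaction input.
; Overlapping its box as PlayerBp enables input, reveals a text prompt and prepares a dialogue widget; leaving hides only the prompt, without disabling input.
; Each press advances the index and shows that line in a Coversacion1 widget while deactivating character movement.
; Pressing past the last line restores movement, removes the widget and resets the index.
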(event `EnhancedInput|/Game/Players/Bp/LP_interaccion`
  (params (ActionValue :type Boolean) (ElapsedSeconds :type "Float (double-precision)") (TriggeredSeconds :type "Float (double-precision)") (InputAction :type "InputAction Object Reference" :default "/Game/Players/Bp/LP_interaccion.LP_interaccion"))
  (bind _dialogue_widget (`self.Dialogue Widget`))
  (bind _index (`self.index`))
  (:`Started`
    (`/Engine/EditorBlueprintResources/StandardMacros.IncrementInt` _index
      (:`  `
        (if (<= _index (`KismetArrayLibrary.Array_LastIndex` (`self.Dialogue Text`)))
          (`/Engine/EditorBlueprintResources/StandardMacros.IsValid` (`self.Dialogue Widget`)
            (:`Is Valid`
              _)
            (:`Is Not Valid`
              (bind _returnvalue (`|CreateWidget` "/Game/Widgest/Mensajes/Coversacion1.Coversacion1_C"))
              (set `self.Dialogue Widget` _returnvalue)))
          (`TextBlock.SetText` (`/Game/Widgest/Mensajes/Coversacion1.DialogueText` (`self.Dialogue Widget`)) (`|GetArrayItem` (`self.Dialogue Text`) (`self.Index`)))
          (`UserWidget.AddToViewport` (`self.Dialogue Widget`) 0)
          (bind _asplayer_bp (cast `/Game/Players/Bp/PlayerBp` (`GameplayStatics.GetPlayerCharacter` 0)))
          (`ActorComponent.Deactivate` (`Character.CharacterMovement` _asplayer_bp))
          (else
            (bind _asplayer_bp_2 (cast `/Game/Players/Bp/PlayerBp` (`GameplayStatics.GetPlayerCharacter` 0)))
            (`ActorComponent.Activate` (`Character.CharacterMovement` _asplayer_bp_2) false)
            (`/Engine/EditorBlueprintResources/StandardMacros.IsValid` _dialogue_widget
              (:`Is Valid`
                (`Widget.RemoveFromParent` _dialogue_widget)
                (set `self.Index` -1)
                (set `self.Dialogue Widget` null)))))))))

(event `self.Box.OnComponentBeginOverlap`
  (params (OverlappedComponent :type "PrimitiveComponent Object Reference") (OtherActor :type "Actor Object Reference") (OtherComp :type "PrimitiveComponent Object Reference") (OtherBodyIndex :type Integer) (bFromSweep :type Boolean) (SweepResult :type "HitResult Structure (by ref)"))
  (cast `/Game/Players/Bp/PlayerBp` OtherActor)
  (`self.EnableInput` (`GameplayStatics.GetPlayerController` 0))
  (`SceneComponent.SetHiddenInGame` (`self.TextRender`) false false)
  (if (`self.ActorHasTag` OtherActor "Player")
    (bind _returnvalue (`|CreateWidget` "/Game/Widgest/Mensajes/Coversacion1.Coversacion1_C"))
    (set `self.Dialogue Widget` _returnvalue)
    (`TextBlock.SetText` (`/Game/Widgest/Mensajes/Coversacion1.DialogueText` (`self.Dialogue Widget`)) (`|GetArrayItem` (`self.Dialogue Text`)))
    (`TextBlock.SetText` (`/Game/Widgest/BpWidgetBienvenido.DialogueText` (`self.Dialogue`)) (`|GetArrayItem` (`self.Dialogue Text`)))))

(event `self.Box.OnComponentEndOverlap`
  (params (OverlappedComponent :type "PrimitiveComponent Object Reference") (OtherActor :type "Actor Object Reference") (OtherComp :type "PrimitiveComponent Object Reference") (OtherBodyIndex :type Integer))
  (cast `/Game/Players/Bp/PlayerBp` OtherActor)
  (`SceneComponent.SetHiddenInGame` (`self.TextRender`) true false))

(fn `UserConstructionScript`)