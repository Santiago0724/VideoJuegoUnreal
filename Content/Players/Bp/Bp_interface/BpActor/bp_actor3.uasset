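; Interactable dialogue actor that shows a text prompt and enables input when PlayerBp enters its box, creating a BpWidgetBienvenido widget for Player-tagged actors.
; The LP_interaccion action steps through DialogueText, deactivating player movement until the lines run out, then restores movement and resets.
; Leaving the box hides the prompt and removes MainWidget, a separate variable from DialogueWidget, without disabling input.
; Recoleccion returns a Nombre entry by TextRow.
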(event `EnhancedInput|/Game/Players/Bp/LP_interaccion`
  (params (ActionValue :type Boolean) (ElapsedSeconds :type "Float (double-precision)") (TriggeredSeconds :type "Float (double-precision)") (InputAction :type "InputAction Object Reference" :default "/Game/Players/Bp/LP_interaccion.LP_interaccion"))
  (bind _index (`self.Index`))
  (:`Started`
    (`/Engine/EditorBlueprintResources/StandardMacros.IncrementInt` _index
      (:`  `
        (if (<= _index (`KismetArrayLibrary.Array_LastIndex` (`self.DialogueText`)))
          (`TextBlock.SetText` (`/Game/Widgest/BpWidgetBienvenido.DialogueText` (`self.DialogueWidget`)) (`|GetArrayItem` (`self.DialogueText`) (`self.Index`)))
          (`UserWidget.AddToViewport` (`self.DialogueWidget`) 0)
          (bind _asplayer_bp (cast `/Game/Players/Bp/PlayerBp` (`GameplayStatics.GetPlayerCharacter` 0)))
          (`ActorComponent.Deactivate` (`Character.CharacterMovement` _asplayer_bp))
          (else
            (bind _asplayer_bp_2 (cast `/Game/Players/Bp/PlayerBp` (`GameplayStatics.GetPlayerCharacter` 0)))
            (`ActorComponent.Activate` (`Character.CharacterMovement` _asplayer_bp_2) false)
            (`Widget.RemoveFromParent` (`self.DialogueWidget`))
            (set `self.Index` -1)))))))

(event `self.Box.OnComponentBeginOverlap`
  (params (OverlappedComponent :type "PrimitiveComponent Object Reference") (OtherActor :type "Actor Object Reference") (OtherComp :type "PrimitiveComponent Object Reference") (OtherBodyIndex :type Integer) (bFromSweep :type Boolean) (SweepResult :type "HitResult Structure (by ref)"))
  (cast `/Game/Players/Bp/PlayerBp` OtherActor)
  (`self.EnableInput` (`GameplayStatics.GetPlayerController` 0))
  (`SceneComponent.SetHiddenInGame` (`self.TextRender`) false false)
  (if (`self.ActorHasTag` OtherActor "Player")
    (bind _returnvalue (`|CreateWidget` "/Game/Widgest/BpWidgetBienvenido.BpWidgetBienvenido_C"))
    (set `self.DialogueWidget` _returnvalue)
    (`TextBlock.SetText` (`/Game/Widgest/BpWidgetBienvenido.DialogueText` (`self.DialogueWidget`)) (`|GetArrayItem` (`self.DialogueText`)))))

(event `self.Box.OnComponentEndOverlap`
  (params (OverlappedComponent :type "PrimitiveComponent Object Reference") (OtherActor :type "Actor Object Reference") (OtherComp :type "PrimitiveComponent Object Reference") (OtherBodyIndex :type Integer))
  (bind _mainwidget (`self.mainWidget`))
  (cast `/Game/Players/Bp/PlayerBp` OtherActor)
  (`SceneComponent.SetHiddenInGame` (`self.TextRender`) true false)
  (`/Engine/EditorBlueprintResources/StandardMacros.IsValid` _mainwidget
    (:`Is Valid`
      (`Widget.RemoveFromParent` _mainwidget))))

(fn `Recoleccion`
  (returns (`Return value` :type Text))
  (bind _textrow (`self.textRow`))
  (return (`|GetArrayItem` (`self.Nombre`) (select `bool` (== _textrow -1) :`false` _textrow))))

(fn `UserConstructionScript`)