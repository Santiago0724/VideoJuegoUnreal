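; Dialogue actor that lets the player step through lines of text with E after entering its Box trigger.
; Overlap enables input, shows a TextRender and creates a Coversacion1 widget; each press displays the next DialogueText entry and deactivates player movement until the lines run out.
; Leaving hides the TextRender and removes MainWidget, not DialogueWidget, and never disables input.
; Recoleccion separately returns a Nombre entry by TextRow.
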(event `Key|E`
  (params (Key :type "Key Structure"))
  (bind _dialoguewidget (`self.DialogueWidget`))
  (bind _index (`self.Index`))
  (:`Pressed`
    (`/Engine/EditorBlueprintResources/StandardMacros.IncrementInt` _index
      (:`  `
        (if (<= _index (`KismetArrayLibrary.Array_LastIndex` (`self.DialogueText`)))
          (`/Engine/EditorBlueprintResources/StandardMacros.IsValid` (`self.DialogueWidget`)
            (:`Is Valid`
              _)
            (:`Is Not Valid`
              (bind _returnvalue (`|CreateWidget` "/Game/Widgest/Mensajes/Coversacion1.Coversacion1_C"))
              (set `self.DialogueWidget` _returnvalue)))
          (`TextBlock.SetText` (`/Game/Widgest/Mensajes/Coversacion1.DialogueText` (`self.DialogueWidget`)) (`|GetArrayItem` (`self.DialogueText`) (`self.Index`)))
          (`UserWidget.AddToViewport` (`self.DialogueWidget`) 0)
          (bind _asplayer_bp (cast `/Game/Players/Bp/PlayerBp` (`GameplayStatics.GetPlayerCharacter` 0)))
          (`ActorComponent.Deactivate` (`Character.CharacterMovement` _asplayer_bp))
          (else
            (bind _asplayer_bp_2 (cast `/Game/Players/Bp/PlayerBp` (`GameplayStatics.GetPlayerCharacter` 0)))
            (`ActorComponent.Activate` (`Character.CharacterMovement` _asplayer_bp_2) false)
            (`/Engine/EditorBlueprintResources/StandardMacros.IsValid` _dialoguewidget
              (:`Is Valid`
                (`Widget.RemoveFromParent` _dialoguewidget)
                (set `self.Index` -1)
                (set `self.DialogueWidget` null)))))))))

(event `self.Box.OnComponentBeginOverlap`
  (params (OverlappedComponent :type "PrimitiveComponent Object Reference") (OtherActor :type "Actor Object Reference") (OtherComp :type "PrimitiveComponent Object Reference") (OtherBodyIndex :type Integer) (bFromSweep :type Boolean) (SweepResult :type "HitResult Structure (by ref)"))
  (cast `/Game/Players/Bp/PlayerBp` OtherActor)
  (`self.EnableInput` (`GameplayStatics.GetPlayerController` 0))
  (`SceneComponent.SetHiddenInGame` (`self.TextRender`) false false)
  (bind _returnvalue (`|CreateWidget` "/Game/Widgest/Mensajes/Coversacion1.Coversacion1_C"))
  (set `self.DialogueWidget` _returnvalue)
  (`TextBlock.SetText` (`/Game/Widgest/Mensajes/Coversacion1.DialogueText` (`self.DialogueWidget`)) (`|GetArrayItem` (`self.DialogueText`))))

(event `self.Box.OnComponentEndOverlap`
  (params (OverlappedComponent :type "PrimitiveComponent Object Reference") (OtherActor :type "Actor Object Reference") (OtherComp :type "PrimitiveComponent Object Reference") (OtherBodyIndex :type Integer))
  (bind _mainwidget (`self.mainWidget`))
  (cast `/Game/Players/Bp/PlayerBp` OtherActor)
  (`SceneComponent.SetHiddenInGame` (`self.TextRender`) true false)
  (`/Engine/EditorBlueprintResources/StandardMacros.IsValid` _mainwidget
    (:`Is Valid`
      (`Widget.RemoveFromParent` _mainwidget))))

(fn `Recoleccion`
  (returns (`Return value` :type Text))
  (bind _textrow (`self.textRow`))
  (return (`|GetArrayItem` (`self.Nombre`) (select `bool` (== _textrow -1) :`false` _textrow))))

(fn `UserConstructionScript`)