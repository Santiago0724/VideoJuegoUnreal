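; Conversation trigger actor that shows a line-by-line dialogue when the player enters its box.
; Overlap enables input, reveals a text render and, for a "Player"-tagged actor, opens a Coversacion1 widget with the first line and deactivates character movement.
; The LP_interaccion input steps through the DialogueText array, then removes the widget, restores movement and resets the index.
; End overlap hides the text and removes MainWidget, a separate variable never assigned here.
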(event `EnhancedInput|/Game/Players/Bp/LP_interaccion`
  (params (ActionValue :type Boolean) (ElapsedSeconds :type "Float (double-precision)") (TriggeredSeconds :type "Float (double-precision)") (InputAction :type "InputAction Object Reference" :default "/Game/Players/Bp/LP_interaccion.LP_interaccion"))
  (bind _index (`self.Index`))
  (:`Started`
    (`/Engine/EditorBlueprintResources/StandardMacros.IncrementInt` _index
      (:`  `
        (if (<= _index (`KismetArrayLibrary.Array_LastIndex` (`self.DialogueText`)))
          (`TextBlock.SetText` (`/Game/Widgest/Mensajes/Coversacion1.DialogueText` (`self.Dialogue Widget`)) (`|GetArrayItem` (`self.DialogueText`) (`self.Index`)))
          (else
            (bind _asplayer_bp (cast `/Game/Players/Bp/PlayerBp` (`GameplayStatics.GetPlayerCharacter` 0)))
            (`ActorComponent.Activate` (`Character.CharacterMovement` _asplayer_bp) false)
            (`Widget.RemoveFromParent` (`self.Dialogue Widget`))
            (set `self.Index` -1)))))))

(event `self.Box.OnComponentBeginOverlap`
  (params (OverlappedComponent :type "PrimitiveComponent Object Reference") (OtherActor :type "Actor Object Reference") (OtherComp :type "PrimitiveComponent Object Reference") (OtherBodyIndex :type Integer) (bFromSweep :type Boolean) (SweepResult :type "HitResult Structure (by ref)"))
  (cast `/Game/Players/Bp/PlayerBp` OtherActor)
  (`self.EnableInput` (`GameplayStatics.GetPlayerController` 0))
  (`SceneComponent.SetHiddenInGame` (`self.TextRender1`) false false)
  (if (`self.ActorHasTag` OtherActor "Player")
    (bind _returnvalue (`|CreateWidget` "/Game/Widgest/Mensajes/Coversacion1.Coversacion1_C"))
    (set `self.Dialogue Widget` _returnvalue)
    (`TextBlock.SetText` (`/Game/Widgest/Mensajes/Coversacion1.DialogueText` (`self.Dialogue Widget`)) (`|GetArrayItem` (`self.DialogueText`)))
    (`UserWidget.AddToViewport` (`self.Dialogue Widget`) 0)
    (bind _asplayer_bp (cast `/Game/Players/Bp/PlayerBp` (`GameplayStatics.GetPlayerCharacter` 0)))
    (`ActorComponent.Deactivate` (`Character.CharacterMovement` _asplayer_bp))))

(event `self.Box.OnComponentEndOverlap`
  (params (OverlappedComponent :type "PrimitiveComponent Object Reference") (OtherActor :type "Actor Object Reference") (OtherComp :type "PrimitiveComponent Object Reference") (OtherBodyIndex :type Integer))
  (bind _mainwidget (`self.mainWidget`))
  (cast `/Game/Players/Bp/PlayerBp` OtherActor)
  (`SceneComponent.SetHiddenInGame` (`self.TextRender1`) true false)
  (`/Engine/EditorBlueprintResources/StandardMacros.IsValid` _mainwidget
    (:`Is Valid`
      (`Widget.RemoveFromParent` _mainwidget))))

(fn `UserConstructionScript`)